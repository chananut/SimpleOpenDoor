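; Trigger-box actor that opens and closes a door while actors are inside it.
; On BeginPlay it copies its start, end, speed, mode and target mesh settings into the CompDooropen component.
; Box overlaps maintain a list of occupants, so the component opens the gate for the first actor in and closes it after the last leaves.
; Each begin overlap also prints a debug string.
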(event OnComponentBeginOverlap(Box)
  (params (OverlappedComponent :type Primitive%20Component%20Object%20Reference) (OtherActor :type Actor%20Object%20Reference) (OtherComp :type Primitive%20Component%20Object%20Reference) (OtherBodyIndex :type Integer) (bFromSweep :type Boolean) (SweepResult :type Hit%20Result%20Structure%20%28by%20ref%29))
  (if (== (Utilities|Array|Length (Variables|Default|GetactorList)) 0)
    (Default|OpenGate (Variables|Default|Getcomp_dooropen)))
  (Utilities|Array|Add (Variables|Default|GetactorList) OtherActor)
  (Development|PrintString "Hello"))

(event OnComponentEndOverlap(Box)
  (params (OverlappedComponent :type Primitive%20Component%20Object%20Reference) (OtherActor :type Actor%20Object%20Reference) (OtherComp :type Primitive%20Component%20Object%20Reference) (OtherBodyIndex :type Integer))
  (Utilities|Array|RemoveItem (Variables|Default|GetactorList) OtherActor)
  (if (== (Utilities|Array|Length (Variables|Default|GetactorList)) 0)
    (Default|CloseGate (Variables|Default|Getcomp_dooropen))))

(event EventBeginPlay
  (bind _comp_dooropen (Variables|Default|Getcomp_dooropen))
  (Variables|/Game/SimpleOpenDoor/comp_dooropen.comp_dooropen_C|Setstart _comp_dooropen (Variables|Default|Getstart))
  (Variables|/Game/SimpleOpenDoor/comp_dooropen.comp_dooropen_C|Setend _comp_dooropen (Variables|Default|Getend))
  (Variables|/Game/SimpleOpenDoor/comp_dooropen.comp_dooropen_C|Setspeed _comp_dooropen (Variables|Default|Getspeed))
  (Variables|/Game/SimpleOpenDoor/comp_dooropen.comp_dooropen_C|Setenum _comp_dooropen (Variables|Default|Getmode))
  (Variables|/Game/SimpleOpenDoor/comp_dooropen.comp_dooropen_C|Setmesh _comp_dooropen (Variables|Default|Gettarget)))

(fn ConstructionScript)